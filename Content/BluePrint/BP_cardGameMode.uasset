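; Game mode for a timed card game that shows the HUD and decides between success and game over.
; BeginPlay resets the timer to its maximum, and a Delay on Tick acts as a one-second countdown that opens the game-over widget at zero.
; Tick also polls the player pawn's correct-card count and opens the success widget when it equals eight.
; Both end screens switch input to UI only.
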(event EventBeginPlay
  (Utilities|FlowControl|Sequence
    (:then_0
      (bind _returnvalue (UserInterface|CreateWidget "/Game/BluePrint/BP_HUD.BP_HUD_C"))
      (bind _output_get (Variables|Default|SetBPW_HUD _returnvalue))
      (UserInterface|Viewport|AddtoViewport _output_get 0))
    (:then_2
      (Variables|Default|SetNew_Time (Variables|Default|GetMax_Time)))))

(event EventTick
  (params (DeltaSeconds :type Float%20%28single-precision%29))
  (Utilities|FlowControl|Sequence
    (:then_0
      (Utilities|FlowControl|Delay 1.0)
      (if (== (Variables|Default|GetNew_Time) 0.0)
        (Utilities|FlowControl|Delay 1.0)
        (CallFunction|GameOver)
        (else
          (Variables|Default|SetNew_Time (Math|Float|Clamp(Float) (- (Variables|Default|GetNew_Time) 1.0) 0.0 (Variables|Default|GetMax_Time))))))
    (:then_1
      (bind _asbp_player (Utilities|Casting|CastToBP_Player (Game|Player|GetPlayerPawn 0)))
      (Math|Integer|CompareInt (Variables|/Game/BluePrint/BP_Player.BP_Player_C|GetCorrecCard _asbp_player) 8
        (:==
          (Utilities|FlowControl|Delay 1.0)
          (CallFunction|Success))))))

(fn ConstructionScript)

(fn GameOver
  (bind _returnvalue (UserInterface|CreateWidget "/Game/BluePrint/BPW_GameOver.BPW_GameOver_C"))
  (UserInterface|Viewport|AddtoViewport _returnvalue 0)
  (Input|SetInputModeUIOnly (Game|GetPlayerController 0) _returnvalue "DoNotLock"))

(fn Success
  (bind _returnvalue (UserInterface|CreateWidget "/Game/BluePrint/BPW_Success.BPW_Success_C"))
  (UserInterface|Viewport|AddtoViewport _returnvalue 0)
  (Input|SetInputModeUIOnly (Game|GetPlayerController 0) _returnvalue "DoNotLock"))