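; BP_Player is a player Blueprint holding simple counter logic in its event graph.
; Every tick it sets CompareNumber to the difference between Compare11 and Compare12.
; It also checks Stack each tick, and when it equals 3, delays half a second, resets it to 0, then after a short delay sets it to 1.
; The construction script is empty.
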(event EventTick
  (params (DeltaSeconds :type Float%20%28single-precision%29))
  (Utilities|FlowControl|Sequence
    (:then_0
      (Variables|Default|SetCompareNumber (- (Variables|Default|GetCompare1_1) (Variables|Default|GetCompare1_2))))
    (:then_1
      (Math|Integer|CompareInt (Variables|Default|GetStack) 3
        (:==
          (Utilities|FlowControl|Delay 0.5)
          (Variables|Default|SetStack 0)
          (Utilities|FlowControl|Delay 0.1)
          (Variables|Default|SetStack 1))))))

(fn ConstructionScript)