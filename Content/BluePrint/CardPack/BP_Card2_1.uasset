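; BP_Card2_1 is a card actor, apparently from a matching game, that removes itself once its pair is matched.
; Each Tick it polls BP_Player to check whether both Compare11 and Compare12 hold this card's value, summing the two booleans as integers.
; On a match it waits briefly, spawns a pixel explosion, destroys itself and increments the player's CorrecCard counter.
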(event EventBeginPlay
  (|CallParentFunction) ; 지금 이 노드는 비활성 상태입니다. \n핀을 끌어서 다른 노드를 연결하면 활성화됩니다.
)

(event Collision|EventActorBeginOverlap
  (params (OtherActor :type Actor%20Object%20Reference)))

(event EventTick
  (params (DeltaSeconds :type Float%20%28single-precision%29))
  (|CallParentFunction 0.0)
  (bind _asbp_player (Utilities|Casting|CastToBP_Player (Game|Player|GetPlayerPawn 0)))
  (Math|Integer|CompareInt (+ (Math|Conversions|ToInteger(Boolean) (== (Variables|/Game/BluePrint/BP_Player.BP_Player_C|GetCompare1_1 _asbp_player) 2)) (Math|Conversions|ToInteger(Boolean) (== (Variables|/Game/BluePrint/BP_Player.BP_Player_C|GetCompare1_2 _asbp_player) 2))) 2
    (:==
      (Utilities|FlowControl|Delay 0.5)
      (Effects|SpawnEmitteratLocation "/Game/Asset/Particles/P_Pixel_Explosion.P_Pixel_Explosion" (Transformation|GetActorLocation))
      (Actor|DestroyActor)
      (bind _asbp_player_2 (Utilities|Casting|CastToBP_Player (Game|Player|GetPlayerPawn 0)))
      (Variables|/Game/BluePrint/BP_Player.BP_Player_C|SetCorrecCard _asbp_player_2 (+ (Variables|/Game/BluePrint/BP_Player.BP_Player_C|GetCorrecCard _asbp_player_2) 1)))))

(fn ConstructionScript
  (|CallParentFunction))