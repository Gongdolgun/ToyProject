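; Base card actor for what appears to be a pair-matching game, handling flips and removal.
; Timelines rotate it out and back at spawn and flip it on click, which passes CardNumber to BP_Player and increments Stack.
; Tick polls the player, flipping back or resetting Compare12 by CompareNumber when Stack is zero.
; When the game mode's NewTime hits zero, it explodes and destroys itself.
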(event EventBeginPlay
  ;[1 1 1] BeginPlay
  (bind _asbp_game_mode (Utilities|Casting|CastToBP_cardGameMode (Game|GetGameMode)))
  (Variables|Default|SetBP_GameMode _asbp_game_mode)
  (Timeline|타임라인_3 Play
    (:Update
      (bind _새_트랙_0 (Timeline|타임라인_2 Play)
        (:Update
          (Transformation|SetActorRotation (Math|Rotator|Lerp(Rotator) "0, 0, 0" (Math|Rotator|MakeRotator (+ (Variables|Default|GetYaw) (Variables|Default|GetSpawnSpinCount)) 0.0 0.0) _새_트랙_0)))))
    (:Finished
      (Timeline|타임라인_2 Reverse))))

(event EventTick
  (params (DeltaSeconds :type Float%20%28single-precision%29))
  ;[1 1 1] Card Flip Flop
  (if (== (Variables|/Game/BluePrint/BP_cardGameMode.BP_cardGameMode_C|GetNew_Time (Variables|Default|GetBP_GameMode)) 0.0)
    (Effects|SpawnEmitteratLocation "/Game/Asset/Particles/P_Pixel_Explosion_Player.P_Pixel_Explosion_Player" (Transformation|GetActorLocation))
    (Actor|DestroyActor)
    (else
      (bind _asbp_player (Utilities|Casting|CastToBP_Player (Game|Player|GetPlayerPawn 0)))
      (Math|Integer|CompareInt (Variables|/Game/BluePrint/BP_Player.BP_Player_C|GetStack _asbp_player)
        (:==
          (bind _asbp_player_2 (Utilities|Casting|CastToBP_Player (Game|Player|GetPlayerPawn 0)))
          (Math|Integer|CompareInt (Variables|/Game/BluePrint/BP_Player.BP_Player_C|GetCompareNumber _asbp_player_2)
            (:>
              (Timeline|타임라인_1 PlayFromStart
                (:Update
                  ;[1 1 1] Flip Card
                  (bind _새_트랙_0 (Timeline|타임라인_0 Reverse)
                    (:Update
                      (Transformation|SetActorRotation (Math|Rotator|Lerp(Rotator) "0, 0, 0" (Math|Rotator|MakeRotator (+ (Variables|Default|GetYaw) (Variables|Default|GetSpawnSpinCount)) 0.0 0.0) _새_트랙_0)))))
                (:Finished
                  (bind _asbp_player_3 (Utilities|Casting|CastToBP_Player (Game|Player|GetPlayerPawn 0) :!label _label))
                  (Variables|/Game/BluePrint/BP_Player.BP_Player_C|SetCompare1_2 _asbp_player_3 51))))
            (:==
              (Utilities|FlowControl|Delay 0.1)
              (goto _label))
            (:<
              (Timeline|타임라인_1 PlayFromStart))))))))

(event MouseInput|EventActorOnClicked
  (params (ButtonPressed :type Key%20Structure))
  ;[1 1 1] Card Flip Flop
  (Utilities|FlowControl|Sequence
    (:then_0
      (bind _asbp_game_mode (Utilities|Casting|CastToBP_cardGameMode (Game|GetGameMode)))
      (Variables|Default|SetBP_GameMode _asbp_game_mode)
      ;[1 1 1] Flip Card
      (bind _새_트랙_0 (Timeline|타임라인_0 PlayFromStart)
        (:Update
          (Transformation|SetActorRotation (Math|Rotator|Lerp(Rotator) "0, 0, 0" (Math|Rotator|MakeRotator (+ (Variables|Default|GetYaw) (Variables|Default|GetSpawnSpinCount)) 0.0 0.0) _새_트랙_0)))))
    (:then_1
      (bind _asbp_player (Utilities|Casting|CastToBP_Player (Game|Player|GetPlayerPawn 0)))
      (Variables|/Game/BluePrint/BP_Player.BP_Player_C|SetCompare1_2 _asbp_player (Variables|Default|GetCardNumber))
      (Variables|/Game/BluePrint/BP_Player.BP_Player_C|SetStack _asbp_player (+ (Variables|/Game/BluePrint/BP_Player.BP_Player_C|GetStack _asbp_player) 1)))))

(fn ConstructionScript)