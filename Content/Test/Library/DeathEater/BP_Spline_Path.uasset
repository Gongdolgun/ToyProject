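; BP_Spline_Path is an actor in the DeathEater test library that builds an arced spline from its own location to a given destination.
; The CreatePath event clears the spline and sets two world-space points, the root location and FinalLoc.
; It gives the endpoints opposite local-space vertical tangents, scaled by their distance and the Curve variable, so the arc grows with path length.
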(event Custom|Create%20Path
  (params (Final%20Loc :type Vector))
  (bind _spline (Variables|Default|GetSpline))
  (bind _defaultsceneroot (Variables|Default|GetDefaultSceneRoot))
  (bind _curve (Variables|Default|GetCurve))
  (bind _returnvalue (Transformation|GetWorldLocation _defaultsceneroot))
  (bind _returnvalue_2 (- _returnvalue Final%20Loc))
  (bind _returnvalue_3 (Math|Vector|VectorLength _returnvalue_2))
  (bind _returnvalue_4 (* _returnvalue_3 _curve))
  (bind _returnvalue_5 (Math|Vector|MakeVector 0.0 0.0 _returnvalue_4))
  (Spline|ClearSplinePoints _spline true)
  (Spline|SetSplinePoints _spline (Utilities|Array|MakeArray _returnvalue Final%20Loc) "World" true)
  (Spline|SetTangentatSplinePoint _spline 0 _returnvalue_5 "Local" true)
  (Spline|SetTangentatSplinePoint _spline 1 (* _returnvalue_5 -1.0) "Local" true))

(event EventBeginPlay)

(event Collision|EventActorBeginOverlap
  (params (OtherActor :type Actor%20Object%20Reference)))

(event EventTick
  (params (DeltaSeconds :type Float%20%28single-precision%29)))

(fn ConstructionScript)