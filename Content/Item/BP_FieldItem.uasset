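; BP_FieldItem is a world item actor that takes its appearance from an item class ID.
; On BeginPlay, a nonzero ItemClassID looks up its ItemClassTable row and asynchronously loads that row's static mesh.
; Weapon-type items are pitched or rolled 90 degrees without waiting for the load.
; Once loaded, the mesh is applied and the sphere component's radius is resized to match its bounds.
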(event EventBeginPlay
  (bind _staticmesh (Variables|Default|GetStaticMesh))
  (if (!= (Variables|Default|GetItemClassID) 0)
    (bind _returnvalue (Utilities|GetDataTableRow "/Game/Item/ItemClassTable.ItemClassTable" (Utilities|String|StringToName (Utilities|String|ToString(Integer) (Variables|Default|GetItemClassID))))
      (:then
        (bind _object (Utilities|AsyncLoadAsset (.StaticMesh (Utilities|Struct|BreakItemClass _returnvalue)))
          (:then
            (switch Utilities|FlowControl|Switch|SwitchonEItemEquipType (.ItemEquipType (Utilities|Struct|BreakItemClass _returnvalue))
              (:NewEnumerator4
                (Transformation|SetActorRelativeRotation "0, 0,90.000000"))))
          (:Completed
            (bind _asstatic_mesh (Utilities|Casting|CastToStaticMesh _object))
            (Components|StaticMesh|SetStaticMesh _staticmesh _asstatic_mesh)
            (Components|Sphere|SetSphereRadius (Variables|Default|GetSphere) (.SphereRadius (Collision|GetComponentBounds _staticmesh)) true)))))))

(fn ConstructionScript)